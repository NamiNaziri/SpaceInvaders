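; Base player controller that handles pausing and death for the player through the core HUD.
; On BeginPlay it adds the keyboard and mouse Enhanced Input mapping context.
; The pause input pauses the game and shows the HUD's pause menu.
; The death event also pauses the game, then has the HUD show the leaderboard entry modal.
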(event Input|EnhancedActionEvents|EnhancedInputActionIA_Pause
  (params (ActionValue :type Boolean) (ElapsedSeconds :type Float%20%28double-precision%29) (TriggeredSeconds :type Float%20%28double-precision%29) (InputAction :type Input%20Action%20Object%20Reference :default "/Game/Player/Input/Actions/IA_Pause.IA_Pause"))
  (:Triggered
    (Game|SetGamePaused true)
    (bind _asbp_core_hud (Utilities|Casting|CastToBP_Core_Hud (HUD|GetHUD)))
    (Default|ShowPauseMenu _asbp_core_hud)))

(event EventBeginPlay
  (Input|AddMappingContext (PlayerController|LocalPlayerSubsystems|GetEnhancedInputLocalPlayerSubsystem) "/Game/Player/Input/Mappings/IMC_Controller_KBM.IMC_Controller_KBM" 0 "(bIgnoreAllPressedKeysUntilRelease=True,bForceImmediately=False)"))

(event EventRecieveonDeath
  (Game|SetGamePaused true)
  (bind _asbp_core_hud (Utilities|Casting|CastToBP_Core_Hud (HUD|GetHUD)))
  (Default|ShowLeaderboardEntryModal _asbp_core_hud))

(fn ConstructionScript)