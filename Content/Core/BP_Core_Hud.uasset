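; BP_Core_Hud is the HUD Blueprint that owns the main menu and pause menu widgets and switches which one has focus.
; On BeginPlay it creates both collapsed in the viewport, then shows the main menu with cursor and UI-only input.
; ShowPauseMenu swaps the focused widget through ClearFocusedWidget and InitFocusedWidget, which toggle visibility, cursor and game-only or UI-only input mode.
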(event Custom|ShowPauseMenu
  (CallFunction|ClearFocusedWidget)
  (Variables|Default|SetCurrentFocusedWidget (Variables|Default|GetWBO_PauseMenu))
  (CallFunction|InitFocusedWidget))

(event Custom|ClearFocusedWidget
  (Variables|/Script/Engine.PlayerController|SetbShowMouseCursor (Variables|Default|GetPlayerController) false)
  (Input|SetInputModeGameOnly (Variables|Default|GetPlayerController) false)
  (Widget|SetVisibility (Variables|Default|GetCurrentFocusedWidget) "Collapsed"))

(event Custom|InitFocusedWidget
  (Variables|/Script/Engine.PlayerController|SetbShowMouseCursor (Variables|Default|GetPlayerController) true)
  (Input|SetInputModeUIOnly (Variables|Default|GetPlayerController) (Variables|Default|GetCurrentFocusedWidget) "DoNotLock" false)
  (Widget|SetVisibility (Variables|Default|GetCurrentFocusedWidget) "Visible"))

(event EventBeginPlay
  (Variables|Default|SetPlayerController (Game|Player|GetOwningPlayerController))
  (bind _initialized_widget (CallFunction|InitializeNewWidget "/Game/UI/Widgets/WBP_MainMenu.WBP_MainMenu_C"))
  (bind _output_get (Variables|Default|SetWBP_MainMenu _initialized_widget))
  (bind _output_get_2 (Variables|Default|SetCurrentFocusedWidget _output_get))
  (Widget|SetVisibility _output_get_2 "Visible")
  (Variables|/Script/Engine.PlayerController|SetbShowMouseCursor (Variables|Default|GetPlayerController) true)
  (Input|SetInputModeUIOnly (Variables|Default|GetPlayerController) (Variables|Default|GetWBP_MainMenu) "DoNotLock" false)
  (bind _initialized_widget_2 (CallFunction|InitializeNewWidget "/Game/UI/Widgets/WBP_PauseMenu.WBP_PauseMenu_C"))
  (Variables|Default|SetWBO_PauseMenu _initialized_widget_2))

(fn ConstructionScript)

(fn InitializeNewWidget
  (params (Class :type User%20Widget%20Class%20Reference))
  (bind _returnvalue (UserInterface|CreateWidget Class (Variables|Default|GetPlayerController)))
  (UserInterface|Viewport|AddtoViewport _returnvalue 0)
  (Widget|SetVisibility _returnvalue "Collapsed")
  (return _returnvalue))