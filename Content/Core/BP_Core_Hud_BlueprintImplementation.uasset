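; HUD Blueprint that owns the player's main HUD, main menu, pause menu and leaderboard entry modal widgets and switches between them.
; BeginPlay creates all four collapsed in the viewport, then shows the main menu with mouse cursor and UI-only input.
; Show events hide the main HUD and focus one widget; Clear events restore the HUD, collapse the focused widget and return to game-only input.
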(event Custom|ShowPauseMenu
  (CallFunction|ClearPlayerMainHud)
  (CallFunction|ClearFocusedWidget)
  (Variables|Default|SetCurrentFocusedWidget (Variables|Default|GetWBP_PauseMenu))
  (CallFunction|InitFocusedWidget))

(event Custom|ClearFocusedWidget
  (Variables|/Script/Engine.PlayerController|SetbShowMouseCursor (Variables|Default|GetPlayerController) false)
  (Input|SetInputModeGameOnly (Variables|Default|GetPlayerController) false)
  (Widget|SetVisibility (Variables|Default|GetCurrentFocusedWidget) "Collapsed"))

(event Custom|InitFocusedWidget
  (Variables|/Script/Engine.PlayerController|SetbShowMouseCursor (Variables|Default|GetPlayerController) true)
  (Input|SetInputModeUIOnly (Variables|Default|GetPlayerController) (Variables|Default|GetCurrentFocusedWidget) "DoNotLock" false)
  (Widget|SetVisibility (Variables|Default|GetCurrentFocusedWidget) "Visible"))

(event Custom|ShowLeaderboardEntryModal
  (CallFunction|ClearPlayerMainHud)
  (CallFunction|ClearFocusedWidget)
  (Variables|Default|SetCurrentFocusedWidget (Variables|Default|GetWBP_LeaderboardEntryModal))
  (CallFunction|InitFocusedWidget))

(event Custom|ShowPlayerMainHud
  (Widget|SetVisibility (Variables|Default|GetWBP_PlayerMainHud) "Visible"))

(event Custom|ClearPlayerMainHud
  (Widget|SetVisibility (Variables|Default|GetWBP_PlayerMainHud) "Collapsed"))

(event Custom|ClearPauseMenu
  (CallFunction|ShowPlayerMainHud)
  (CallFunction|ClearFocusedWidget))

(event Custom|ClearLeaderboardEntryModal
  (CallFunction|ShowPlayerMainHud)
  (CallFunction|ClearFocusedWidget))

(event Custom|ClearMainMenu
  (CallFunction|ShowPlayerMainHud)
  (CallFunction|ClearFocusedWidget))

(event EventBeginPlay
  (Variables|Default|SetPlayerController (Game|Player|GetOwningPlayerController))
  (bind _initialized_widget (CallFunction|InitializeNewWidget "/Game/UI/Widgets/WBP_PlayerMainHud.WBP_PlayerMainHud_C"))
  (Variables|Default|SetWBP_PlayerMainHud _initialized_widget)
  (bind _initialized_widget_2 (CallFunction|InitializeNewWidget "/Game/UI/Widgets/WBP_MainMenu.WBP_MainMenu_C"))
  (bind _output_get (Variables|Default|SetWBP_MainMenu _initialized_widget_2))
  (bind _output_get_2 (Variables|Default|SetCurrentFocusedWidget _output_get))
  (Widget|SetVisibility _output_get_2 "Visible")
  (Variables|/Script/Engine.PlayerController|SetbShowMouseCursor (Variables|Default|GetPlayerController) true)
  (Input|SetInputModeUIOnly (Variables|Default|GetPlayerController) (Variables|Default|GetWBP_MainMenu) "DoNotLock" false)
  (bind _initialized_widget_3 (CallFunction|InitializeNewWidget "/Game/UI/Widgets/WBP_PauseMenu.WBP_PauseMenu_C"))
  (Variables|Default|SetWBP_PauseMenu _initialized_widget_3)
  (bind _initialized_widget_4 (CallFunction|InitializeNewWidget "/Game/UI/Widgets/WBP_LeaderboardEntryModal.WBP_LeaderboardEntryModal_C"))
  (Variables|Default|SetWBP_LeaderboardEntryModal _initialized_widget_4))

(fn ConstructionScript)

(fn InitializeNewWidget
  (params (Class :type User%20Widget%20Class%20Reference))
  (bind _returnvalue (UserInterface|CreateWidget Class (Variables|Default|GetPlayerController)))
  (UserInterface|Viewport|AddtoViewport _returnvalue 0)
  (Widget|SetVisibility _returnvalue "Collapsed")
  (return _returnvalue))